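; AI character that races to fetch a thrown toy and shows its name and score above its head.
; It registers with GM_AIGame on BeginPlay, optionally randomizes its walk speed, and smoothly turns toward the player while waiting.
; ChaseToy uses AIMoveTo unless flagged to sit out; reaching the toy stops every listed AI and resets them to waiting.
; The catcher then updates its nametag and the HUD, coloring the top scorer green and others red.
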(event Custom|UpdateWidgets
  (params (ToyShape :type EObjectShape%20Enum :default "Cube"))
  (Variables|Default|SetInObjectShape ToyShape)
  ;[1 1 1] Set appropriate score derived from object shape in UI
  (CallFunction|UpdateNametag)
  (CallFunction|UpdateTextColour (Class|AIGameAICharacter|GetScore))
  (Default|UpdateHud (Variables|Default|GetGameMode)))

(event EventBeginPlay
  ;[1 1 1] Initialize the list of all the AI characters and pass that list to game mode, to avoid calling "get all actors of class", and in case
  (Utilities|FlowControl|Sequence
    (:then_0
      (bind _output_get (Variables|Default|SetGameMode (.AsGM%20AIGame (Utilities|Casting|CastToGM_AIGame (Game|GetGameMode)))))
      (Default|AddtoAICharacterList _output_get self))
    (:then_1
      (bind _aswbp_ai (Utilities|Casting|CastToWBP_AI (UserInterface|GetUserWidgetObject (Variables|Default|GetPlayerNameWidget))))
      (Variables|Default|SetAboveHeadWidjet _aswbp_ai))
    (:then_2
      ;[1 1 1] In case the AI character speed should be random, initialise it
      (Variables|/Script/Engine.CharacterMovementComponent|SetMaxWalkSpeed (Variables|Character|GetCharacterMovement) (Math|Float|SelectFloat (Math|Random|RandomFloatinRange 1e+02 (Class|CharacterMovementComponent|GetMaxAcceleration (Variables|Character|GetCharacterMovement))) (Variables|SpeedSettings|GetCharacterSpeed) (Variables|SpeedSettings|GetIsSpeedRandom))))
    (:then_3
      (CallFunction|UpdateNametag))))

(event EventTick
  (params (DeltaSeconds :type Float%20%28single-precision%29))
  ;[1 1 1] Check if the AI characters should look at the player character
  (if (Variables|Behaviour|GetIsWaiting)
    (CallFunction|RotateAItoPawn DeltaSeconds)))

(event EventChaseToy
  (params (InToy :type BP%20Toy%20Object%20Reference))
  ;[1 1 1] If this AI is the one who shouldn't start chasing the toy, let him have a rest till the next throw =)
  (if (not (Variables|Default|GetbShouldRemainWaiting))
    (Variables|Behaviour|SetIsWaiting false)
    (Variables|Default|SetInObjectShape (Variables|/Script/AIGame.AIGameToy|GetShape InToy))
    (AI|AIMoveTo (Pawn|GetController) self "0, 0, 0" InToy 1e+01 false
      (:OnSuccess
        (Utilities|FlowControl|Sequence
          (:then_0
            (CallFunction|UpdateWidgets (Variables|Default|GetInObjectShape)))
          (:then_1
            ;[1 1 1] When an AI character reaches the toy and takes it all AI characters should stop and start waiting reseting their values to defaults
            (for _array_element (Variables|/Game/GameMode/GM_AIGame.GM_AIGame_C|GetAICharacterList (Variables|Default|GetGameMode))
              (AI|Navigation|StopMovement (Pawn|GetController _array_element))
              (Variables|BP_AI_Character_C|SetIsWaiting _array_element true)
              (Variables|BP_AI_Character_C|SetbShouldRemainWaiting _array_element false))))))))

(fn ConstructionScript)

(fn RotateAItoPawn
  (params (DeltaTime :type Float%20%28double-precision%29) (InPlayerIndex :type Integer))
  (Transformation|SetActorRotation (Math|Rotator|Lerp(Rotator) (Transformation|GetActorRotation) (Math|Conversions|RotationFromXVector (- (Transformation|GetActorLocation (Game|GetPlayerCharacter InPlayerIndex)) (Transformation|GetActorLocation))) (* DeltaTime 1e+01) true)))

(fn UpdateNametag
  (bind _aswbp_ai (Utilities|Casting|CastToWBP_AI (UserInterface|GetUserWidgetObject (Variables|Default|GetPlayerNameWidget))))
  (Default|SetPlayerName _aswbp_ai (Utilities|Text|ToText(String) (Utilities|String|Append (Utilities|String|ToString(Name) (Variables|Default|GetCharacterName)) "  " (Utilities|String|ToString(Integer) (Class|AIGameAICharacter|GetScore))))))

(fn UpdateTextColour
  (params (MyScore :type Integer))
  (bind _gamemode (Variables|Default|GetGameMode))
  (bind _aicharacterlist (Variables|/Game/GameMode/GM_AIGame.GM_AIGame_C|GetAICharacterList _gamemode))
  (for (_array_element _array_index) _aicharacterlist
    (Default|ChangeTextColor (Variables|BP_AI_Character_C|GetAboveHeadWidjet _array_element) (Utilities|Struct|MakeSlateColor "(R=1.000000,G=0.000000,B=0.000000,A=1.000000)"))
    (if (>= (Class|AIGameAICharacter|GetScore _array_element) (LocalVariables|GetMaxValue))
      (LocalVariables|SetMaxValue (Class|AIGameAICharacter|GetScore _array_element))
      (LocalVariables|SetMaxIndex _array_index)))
  (Default|ChangeTextColor (Variables|BP_AI_Character_C|GetAboveHeadWidjet (Utilities|Array|Get(acopy) _aicharacterlist (LocalVariables|GetMaxIndex))) (Utilities|Struct|MakeSlateColor "(R=0.000000,G=1.000000,B=0.000000,A=1.000000)")))