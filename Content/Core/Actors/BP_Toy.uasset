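; BP_Toy is a thrown toy actor that AI characters chase, using a cube or sphere mesh set through an overridden C++ shape event.
; With multiple AI in the GM_AIGame list, CalculateDistance flags the slowest to reach the hit location, by distance over speed, as waiting.
; It then sends every AI a chase interface message.
; An overlap with a near-zero hit location counts as a direct hit and updates that AI's widgets.
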(event Custom|CallAIChaiseMe
  ;[1 1 1] Tell all AI characters to start chasing the toy through blueprint interface, but one will not as it shoud Remain Waiting
  (for _array_element (Variables|/Game/GameMode/GM_AIGame.GM_AIGame_C|GetAICharacterList (Variables|Default|GetGameMode))
    (Class|BPIChaseToy|ChaseToy(Message) _array_element self)))

(event EventBeginPlay
  ;[1 1 1] Get game mode to avoid get all actors of class in future
  (Variables|Default|SetGameMode (.AsGM%20AIGame (Utilities|Casting|CastToGM_AIGame (Game|GetGameMode)))))

(event EventOnComponentOverlap
  (params (OtherActor :type Actor%20Object%20Reference))
  ;[1 1 1] In the situation we throw a toy directly at the AI actor
  (if (Math|Vector|VectorIsNearlyZero (Class|AIGameToy|GetHitLocation))
    (bind _asbp_ai_character (Utilities|Casting|CastToBP_AI_Character OtherActor))
    (Default|UpdateWidgets _asbp_ai_character (Variables|Default|GetShape))))

(event EventSetObjectShape
  (params (InShape :type EObjectShape%20Enum :default "Cube"))
  (bind _staticmeshcomponent (Variables|Default|GetStaticMeshComponent))
  ;[1 1 1] Override C++ Event to set an appropriate static mesh for Toy object
  (bind _output_get (Variables|Default|SetShape InShape))
  (switch Utilities|FlowControl|Switch|SwitchonEObjectShape _output_get
    (:Cube
      (Components|StaticMesh|SetStaticMesh _staticmeshcomponent "/Game/Core/Actors/Shapes/Shape_Cube.Shape_Cube"))
    (:Sphere
      (Components|StaticMesh|SetStaticMesh _staticmeshcomponent "/Game/Core/Actors/Shapes/Shape_Sphere.Shape_Sphere"))))

(event EventCalculateDistance
  (bind _gamemode (Variables|Default|GetGameMode))
  (bind _aicharacterlist (Variables|/Game/GameMode/GM_AIGame.GM_AIGame_C|GetAICharacterList _gamemode))
  ;[1 1 1] Calculate distance if we have more than one AI character
  (if (> (Utilities|Array|Length _aicharacterlist) 1)
    (for (_array_element _array_index) _aicharacterlist
      ;[1 1 1] if time of this AI character is more than one of the previous, get its index
      (if (> (/ (Math|Vector|Distance(Vector) (Transformation|GetActorLocation _array_element) (Class|AIGameToy|GetHitLocation)) (Variables|/Game/Core/AI/BP_AI_Character.BP_AI_Character_C|GetCharacterSpeed _array_element)) (Variables|Default|GetTimeTillToy))
        (Variables|Default|SetTimeTillToy (/ (Math|Vector|Distance(Vector) (Transformation|GetActorLocation _array_element) (Class|AIGameToy|GetHitLocation)) (Variables|/Game/Core/AI/BP_AI_Character.BP_AI_Character_C|GetCharacterSpeed _array_element)))
        ;[1 1 1] Get the index of the slowest AI character
        (Variables|Default|SetAIIndexToStop _array_index)))
    ;[1 1 1] Disable movement of the slowest AI character
    (Variables|/Game/Core/AI/BP_AI_Character.BP_AI_Character_C|SetbShouldRemainWaiting (Utilities|Array|Get(acopy) _aicharacterlist (Variables|Default|GetAIIndexToStop)) true)
    (CallFunction|CallAIChaiseMe)))

(fn ConstructionScript)