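; Game mode for a timed AI match that tracks registered AI characters and their scores and declares a winner.
; BeginPlay takes the round duration from GI_AIGame, creates the HUD and fills in the AI name and score list once after a short delay.
; Tick watches the HUD's end flag, then swaps in the end screen, hides overhead widgets, pauses and shows the top scorer or a dead heat.
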(event Custom|AddToAICharacterList
  (params (InAICharacter :type BP%20AI%20Character%20Object%20Reference))
  ;[1 1 1] Event is called OnBeginPlay of AI characters
  (Utilities|Array|Add (Variables|Default|GetAICharacterList) InAICharacter))

(event Custom|OnEndGame
  (bind _champions (CallFunction|GetChampionIndexes))
  ;[1 1 1] Implement final logics when the game is finished
  (bind _returnvalue (UserInterface|CreateWidget "/Game/UI/WBP_EndGame.WBP_EndGame_C"))
  (bind _output_get (Variables|Widgets|SetEndGameWidget _returnvalue))
  (UserInterface|Viewport|AddtoViewport _output_get 0)
  (Widget|RemovefromParent (Variables|Widgets|GetHUDWidget))
  (CallFunction|RemoveAIWidgets)
  (Game|SetGamePaused true)
  (if (> (Utilities|Array|Length _champions) 1)
    (Default|SetResultingText (Variables|Widgets|GetEndGameWidget) "Dead Heat")
    (else
      (Default|SetResultingText (Variables|Widgets|GetEndGameWidget) (CallFunction|GetChampionText (Utilities|Array|Get(acopy) (Variables|Default|GetAICharacterList) (Utilities|Array|Get(acopy) _champions)))))))

(event EventBeginPlay
  ;[1 1 1] Initialise main HUD widget
  (Utilities|FlowControl|Sequence
    (:then_0
      (bind _asgi_aigame (Utilities|Casting|CastToGI_AIGame (Game|GetGameInstance)))
      (Variables|Default|SetTimeToEnd (Variables|/Game/GI_AIGame.GI_AIGame_C|GetRoundDuration _asgi_aigame)))
    (:then_1
      (bind _returnvalue (UserInterface|CreateWidget "/Game/UI/WBP_HUD.WBP_HUD_C"))
      (bind _output_get (Variables|Widgets|SetHUDWidget _returnvalue))
      (Variables|/Game/UI/WBP_HUD.WBP_HUD_C|SetTime _output_get (Variables|Default|GetTimeToEnd))
      (UserInterface|Viewport|AddtoViewport _output_get 0))
    (:then_2
      (Utilities|FlowControl|Delay 0.5)
      (CallFunction|UpdateHud))))

(event EventTick
  (params (DeltaSeconds :type Float%20%28single-precision%29))
  ;[1 1 1] Implement final logics when the game is finished
  (if (Variables|/Game/UI/WBP_HUD.WBP_HUD_C|GetShouldEndGame (Variables|Widgets|GetHUDWidget))
    (CallFunction|OnEndGame)))

(fn ConstructionScript)

(fn UpdateHud
  (bind _hudwidget (Variables|Widgets|GetHUDWidget))
  (Variables|Default|SetTempString "")
  (for _array_element (Variables|Default|GetAICharacterList)
    (Variables|Default|SetTempString (Utilities|String|Append (Variables|Default|GetTempString) (Utilities|String|ToString(Name) (Variables|/Script/AIGame.AIGameAICharacter|GetCharacterName _array_element)) "   " (Utilities|String|ToString(Integer) (Class|AIGameAICharacter|GetScore _array_element)) " 
")))
  (Variables|/Game/UI/WBP_HUD.WBP_HUD_C|SetInAINames _hudwidget (Utilities|Text|ToText(String) (Variables|Default|GetTempString)))
  (Default|WriteAIData _hudwidget))

(fn RemoveAIWidgets
  (for _array_element (Variables|Default|GetAICharacterList)
    (Widget|RemovefromParent (Variables|/Game/Core/AI/BP_AI_Character.BP_AI_Character_C|GetAboveHeadWidjet _array_element))
    (Widget|SetVisibility (Variables|/Game/Core/AI/BP_AI_Character.BP_AI_Character_C|GetAboveHeadWidjet _array_element) "Collapsed")))

(fn GetChampionIndexes
  (for _array_element (Variables|Default|GetAICharacterList)
    (if (> (Class|AIGameAICharacter|GetScore _array_element) (LocalVariables|GetMaxScore))
      (LocalVariables|SetMaxScore (Class|AIGameAICharacter|GetScore _array_element))))
  (for (_array_element_2 _array_index) (Variables|Default|GetAICharacterList)
    (if (== (Class|AIGameAICharacter|GetScore _array_element_2) (LocalVariables|GetMaxScore))
      (Utilities|Array|Add (LocalVariables|GetChampionsIndexes) _array_index)))
  (return (LocalVariables|GetChampionsIndexes)))

(fn GetChampionText
  (params (InAiCharacter :type BP%20AI%20Character%20Object%20Reference))
  (return (Utilities|Text|ToText(String) (Utilities|String|Append "Winner is " (Utilities|String|ToString(Name) (Variables|/Script/AIGame.AIGameAICharacter|GetCharacterName InAiCharacter)) " gets " (Utilities|String|ToString(Integer) (Class|AIGameAICharacter|GetScore InAiCharacter)) " points"))))